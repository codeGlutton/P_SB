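; Title-screen game mode that builds the player setup view model and opens the main title widget.
; OpenTitleWidget initializes the view model with manager and athlete data and customizing enabled, then shows WBP_MainScene with UI-only input and a visible cursor.
; Network and web-network bind hooks are called on open, and unbind hooks on EndPlay, but all are empty stubs.
; The PlayerSelectPanel view-model connection is disconnected and never runs.
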(event `self.ReceiveBeginPlay`)

(event `self.ReceiveEndPlay`
  (params (EndPlayReason :type "EEndPlayReason Enum" :default "Destroyed"))
  (`self.UnbindNetworkSubsystem`)
  (`self.UnbindWebNetworkSubsystem`))

(event `OpenTitleWidget`
  (params (SelectManagers :type "Array of SBCustomizing Interface (by ref)") (CreateManager :type "SBCustomizing Interface") (CreateAthlete :type "SBCustomizing Interface"))
  (bind _returnvalue (`GameplayStatics.GetPlayerController` 0))
  (bind _returnvalue_2 (`|GenericCreateObject` "/Script/C_SB.SBPlayerSetupViewModel"))
  (bind _output_get (set `self.PlayerSetupViewModel` _returnvalue_2))
  (`SBPlayerSetupViewModel.InitViewModel` _output_get SelectManagers CreateManager CreateAthlete true)
  (`self.BindNetworkSubsystem`)
  (`self.BindWebNetworkSubsystem`)
  (bind _returnvalue_3 (`|CreateWidget` "/Game/SB/Blueprint/UI/Scene/WBP_MainScene.WBP_MainScene_C"))
  (`UserWidget.AddToViewport` _returnvalue_3 0)
  (`WidgetBlueprintLibrary.SetInputMode_UIOnlyEx` _returnvalue null "LockAlways")
  (set `PlayerController.bShowMouseCursor` true _returnvalue))

(event `BindNetworkSubsystem`
  (`self.PlayerSetupViewModel`
    (:`then`)
    (:`else`)))

(event `UnbindNetworkSubsystem`
  (`self.PlayerSetupViewModel`
    (:`then`)
    (:`else`)))

(event `BindWebNetworkSubsystem`)

(event `UnbindWebNetworkSubsystem`)

(fn `UserConstructionScript`)